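; BP_ChessTile is a chess board tile that shows its state through a Paper2D sprite.
; Cursor-over events on its Box component switch the sprite to the hovered look and back to the default when the cursor leaves.
; A clicked-sprite function is also defined, but nothing in this Blueprint calls it.
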(event `self.ReceiveBeginPlay`)

(event `self.ReceiveTick`
  (params (DeltaSeconds :type "Float (single-precision)")))

(event `self.Box.OnBeginCursorOver`
  (params (TouchedComponent :type "PrimitiveComponent Object Reference"))
  (`self.SetHoveredSprite`))

(event `self.Box.OnEndCursorOver`
  (params (TouchedComponent :type "PrimitiveComponent Object Reference"))
  (`self.SetDefaultSprite`))

(fn `SetClickedSprite`
  (`PaperSpriteComponent.SetSprite` (`self.PaperSprite`) (`self.ChessTileClickedSprite`)))

(fn `SetDefaultSprite`
  (`PaperSpriteComponent.SetSprite` (`self.PaperSprite`) (`self.ChessTileDefaultSprite`)))

(fn `SetHoveredSprite`
  (`PaperSpriteComponent.SetSprite` (`self.PaperSprite`) (`self.ChessTileHoveredSprite`)))

(fn `UserConstructionScript`)