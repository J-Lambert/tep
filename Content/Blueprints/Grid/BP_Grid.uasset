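; Grid actor that builds a rectangular field of square tiles as instances of one flat bordered mesh.
; SpawnGrid clears old instances, snaps the center to tile size, derives a corner, then places tiles scaled by the mesh size from the shape DataTable.
; With UseEnvironment, a box trace at each location keeps only tiles that hit something.
; The construction script's SpawnGrid call is disconnected, so it never runs.
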(fn `CalculateCenterAndBottomLeft`
  (returns (Center :type "Vector Structure") (BottomLeft :type "Vector Structure"))
  (locals (C :type "Vector Structure" :default (0.0 0.0 0.0)))
  (bind (_gridtilecount_x _gridtilecount_y) (break `IntPoint` (`self.GridTileCount`)))
  (set `local.C` (`/Game/Blueprints/Utilities/BFL_Utilities.SnapVectorToVector` (`self.GridCenterLocation`) (`KismetMathLibrary.Conv_DoubleToVector` (`self.GridTileSize`))))
  (return (`local.C`) (- (`local.C`) (* (/ (- (`self.GridTileCount`) (`KismetMathLibrary.MakeVector2D` (`KismetMathLibrary.SelectInt` 0 1 (`/Game/Blueprints/Utilities/BFL_Utilities.IsIntEven` _gridtilecount_x)) (`KismetMathLibrary.SelectInt` 0 1 (`/Game/Blueprints/Utilities/BFL_Utilities.IsIntEven` _gridtilecount_y)))) 2.0) (`self.GridTileSize`)))))

(fn `DestroyGrid`
  (`InstancedStaticMeshComponent.ClearInstances` (`self.InstancedStaticMesh`)))

(fn `GetCurrentShapeData`
  (returns (ReturnValue :type "/Game/Blueprints/Grid/S_GridShapeData Structure"))
  (bind _returnvalue (`|GetDataTableRow` "/Game/Blueprints/Grid/DT_GridShapeData.DT_GridShapeData" "Square")
    (:`then`
      (return _returnvalue))))

(fn `GetTileLocationFromGridIndex`
  (params (GridIndex :type "IntPoint Structure"))
  (returns (TileLocation :type "Vector Structure"))
  (return (+ (`self.GridTopLeftCornerLocation`) (* (`self.GridTileSize`) (`KismetMathLibrary.MakeVector` (`KismetMathLibrary.Conv_IntToDouble` GridIndex_X) (`KismetMathLibrary.Conv_IntToDouble` GridIndex_Y))))))

(fn `SpawnGrid`
  (params (CenterLocation :type "Vector Structure") (TileSize :type "Float (double-precision)") (TileCount :type "IntPoint Structure") (UseEnvironment :type Boolean))
  (locals (X :type Integer) (Y :type Integer) (TileTransform :type "Transform Structure") (Index :type "IntPoint Structure"))
  (bind (_gridtilecount_x _gridtilecount_y) (break `IntPoint` (`self.GridTileCount`)))
  (bind _gridtilecount_x_2 (break `IntPoint` (`self.GridTileCount`)))
  (bind (_returnvalue_x _returnvalue_y) (`KismetMathLibrary.BreakVector2D` (/ (`self.GridTileSize`) (`.MeshSize_13_AC4A01224FC4851993D6A6A1DFC19EF0` (break `/Game/Blueprints/Grid/S_GridShapeData` (`self.GetCurrentShapeData`))))))
  (set `self.GridCenterLocation` CenterLocation)
  (set `self.GridTileSize` TileSize)
  (set `self.GridTileCount` TileCount)
  (`self.DestroyGrid`)
  (`StaticMeshComponent.SetStaticMesh` (`self.InstancedStaticMesh`) "/Game/Blueprints/Grid/Square/SM_Grid_SquareFlat.SM_Grid_SquareFlat")
  (`PrimitiveComponent.SetMaterial` (`self.InstancedStaticMesh`) 0 "/Game/Materials/M_Grid_Flat_Border.M_Grid_Flat_Border")
  (bind (_center _bottomleft) (`self.CalculateCenterAndBottomLeft`))
  (set `self.GridCenterLocation` _center)
  (set `self.GridTopLeftCornerLocation` _bottomleft)
  (for _index (range _gridtilecount_x_2)
    (set `local.X` _index)
    (for _index_2 (range _gridtilecount_y)
      (set `local.Y` _index_2)
      (set `local.Index` (make `IntPoint` (`local.X`) (`local.Y`)))
      (bind _output_get (set `local.TileTransform` (`KismetMathLibrary.MakeTransform` (+ (`self.GetTileLocationFromGridIndex` (`local.Index`)) (0.0 0.0 0.01)) (struct) (`KismetMathLibrary.MakeVector` _returnvalue_x _returnvalue_y 1.0))))
      (if (`local.UseEnvironment`)
        (bind _hitsomething (`self.TraceForGround` (.location _output_get)))
        (if _hitsomething
          (`InstancedStaticMeshComponent.AddInstance` (`self.InstancedStaticMesh`) (`local.TileTransform`) true))
        (else
          (`InstancedStaticMeshComponent.AddInstance` (`self.InstancedStaticMesh`) (`local.TileTransform`) true))))))

(fn `TraceForGround`
  (params (Location :type "Vector Structure"))
  (returns (HitSomething :type Boolean))
  (bind _outhits (`KismetSystemLibrary.BoxTraceMulti` Location Location (`KismetMathLibrary.Conv_DoubleToVector` (/ (`self.GridTileSize`) 3.0)) (struct) "TraceTypeQuery3"))
  (if (> (`KismetArrayLibrary.Array_Length` _outhits) 0)
    (return true)
    (else
      (return false))))

(fn `UserConstructionScript`)