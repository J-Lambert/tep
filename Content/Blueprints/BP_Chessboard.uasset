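; BP_Chessboard is an actor that spawns a checkerboard grid of tile actors at BeginPlay, sized by Width and Height.
; Each row swaps the order of MainTile and AlternateTile by index parity, and SpawnRowOfTiles alternates them across the columns.
; SpawnTileAtLocation places tiles at spacing-based world X and negative Y, independent of the board's own transform.
; NumTiles is set to Width plus Height, not their product, and is unused here.
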(event `self.ReceiveBeginPlay`
  (`self.SetNumTiles`)
  (for _index (range (`self.Height`))
    (set `self.TileYPos` (* (* _index (`self.TileYSpacing`)) -1.0))
    (if (`KismetMathLibrary.Conv_IntToBool` (mod _index 2))
      (`self.SpawnRowOfTiles` (`self.MainTile`) (`self.AlternateTile`))
      (else
        (`self.SpawnRowOfTiles` (`self.AlternateTile`) (`self.MainTile`))))))

(fn `SetNumTiles`
  (set `self.NumTiles` (+ (`self.Width`) (`self.Height`))))

(fn `SpawnRowOfTiles`
  (params (FirstTile :type "/Game/Blueprints/BP_ChessTile Class Reference") (SecondTile :type "/Game/Blueprints/BP_ChessTile Class Reference"))
  (for _index (range (`self.Width`))
    (set `self.TileXPos` (* _index (`self.TileXSpacing`)))
    (if (`KismetMathLibrary.Conv_IntToBool` (mod _index 2))
      (`self.SpawnTileAtLocation` FirstTile)
      (else
        (`self.SpawnTileAtLocation` SecondTile)))))

(fn `SpawnTileAtLocation`
  (params (SpawnedTile :type "/Game/Blueprints/BP_ChessTile Class Reference"))
  (`|SpawnActorFromClass` SpawnedTile (`KismetMathLibrary.MakeTransform` (`KismetMathLibrary.MakeVector` (`self.TileXPos`) (`self.TileYPos`))) "Undefined" "MultiplyWithRoot" null null))

(fn `UserConstructionScript`)