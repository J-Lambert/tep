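; BP_Player is the player Blueprint that handles mouse clicks on chess tiles.
; On BeginPlay it adds the IMC_Combat Enhanced Input mapping context to its player controller.
; Pressing IA_Click traces under the cursor on Visibility, stores any hit BP_ChessTile as ClickedTile and shows its clicked sprite.
; Releasing switches the stored tile to its hovered sprite.
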(event `self.ReceiveBeginPlay`
  (bind _asplayer_controller (cast `PlayerController` (`self.GetController`)))
  (`EnhancedInputSubsystemInterface.AddMappingContext` (pcsubsystem `EnhancedInputLocalPlayerSubsystem` _asplayer_controller) "/Game/Input/IMC_Combat.IMC_Combat" 0 (struct)))

(event `EnhancedInput|/Game/Input/IA_Click`
  (params (ActionValue :type Boolean) (ElapsedSeconds :type "Float (double-precision)") (TriggeredSeconds :type "Float (double-precision)") (InputAction :type "InputAction Object Reference" :default "/Game/Input/IA_Click.IA_Click"))
  (bind (_bblockinghit _binitialoverlap _time _distance _location _impactpoint _normal _impactnormal _physmat _hitactor) (`GameplayStatics.BreakHitResult` (`PlayerController.GetHitResultUnderCursorByChannel` (`GameplayStatics.GetPlayerController` 0) "TraceTypeQuery1" true)))
  (:`Started`
    (if _bblockinghit
      (bind _asbp_chess_tile (cast `/Game/Blueprints/BP_ChessTile` _hitactor))
      (set `self.ClickedTile` _asbp_chess_tile)
      (`/Game/Blueprints/BP_ChessTile.SetClickedSprite` _asbp_chess_tile)))
  (:`Completed`
    (`/Game/Blueprints/BP_ChessTile.SetHoveredSprite` (`self.ClickedTile`))))

(fn `UserConstructionScript`)